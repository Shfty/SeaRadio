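; Sea surface plane actor that renders an animated heightmap for its material and answers height queries at world locations.
; Construction and BeginPlay create a dynamic material instance from SeaParameters and a grayscale render target bound as its heightmap texture.
; Each tick redraws the heightmap material into the target, then reads it back to a CPU buffer through C++.
; GetHeightAtWorldLocation bilinearly samples that buffer, applying zero point and height multiplier.
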(event Custom|Setup
  ;[1 1 1] Setup handler
  (bind _seaplanemid (CallFunction|SetupSeaPlaneMID))
  (bind _heightmaprendertarget (CallFunction|SetupHeightmapRenderTarget))
  (Rendering|Material|SetTextureParameterValue _seaplanemid "Heightmap Texture" _heightmaprendertarget)
  (CallFunction|DrawHeightmap))

(event EventTick
  (params (DeltaSeconds :type Float%20%28single-precision%29))
  (bind _heightmaprendertarget (Variables|Default|GetHeightmapRenderTarget))
  ;[1 1 1] Tick handler
  (Utilities|FlowControl|Sequence
    (:then_0
      (CallFunction|DrawHeightmap))
    (:then_1
      ;[1 1 1] Use C++ to read floating point color array back from render texture for later use
      (Utilities|IsValid _heightmaprendertarget
        (:Is%20Valid
          (bind _returnvalue (Class|RenderTextureFunctionLibrary|ReadLinearPixelBuffer _heightmaprendertarget))
          (Variables|Default|SetHeightmapReadback _returnvalue))))))

(event EventBeginPlay
  ;[1 1 1] BeginPlay handler
  ;[1 1 1] Perform setup for in-game / packaged build usage
  (CallFunction|Setup))

(fn ConstructionScript
  ;[1 1 1] Perform setup for editor usage
  (CallFunction|Setup))

(fn GetHeightatWorldLocation
  (params (Location :type Vector))
  (bind _heightmaprendertarget (Variables|Default|GetHeightmapRenderTarget))
  (bind _seaparameters (Variables|Default|GetSeaParameters))
  (bind _plane (Variables|Default|GetPlane))
  (bind _plane_2 (Variables|Default|GetPlane))
  (bind (_heightmultiplier _zeropoint) (Utilities|Struct|BreakSeaPlaneParameters _seaparameters))
  (bind _returnvalue (Transformation|GetWorldLocation _plane))
  (bind _max (Components|StaticMesh|GetLocalBounds _plane_2))
  (bind (_width _height) (Class|CanvasRenderTarget2D|GetSize _heightmaprendertarget))
  (bind _relativescale3d (Variables|/Script/Engine.SceneComponent|GetRelativeScale3D _plane_2))
  (bind _returnvalue_2 (* _max _relativescale3d))
  (bind _returnvalue_3 (- _returnvalue _returnvalue_2))
  (bind _returnvalue_4 (* _returnvalue_2 2.0))
  (bind _returnvalue_5 (- Location _returnvalue_3))
  (bind _returnvalue_6 (/ _returnvalue_5 _returnvalue_4))
  (bind (_x _y) (Math|Vector|BreakVector _returnvalue_6))
  (Utilities|IsValid _heightmaprendertarget
    (:Is%20Valid
      (bind _returnvalue_7 (Class|RenderTextureFunctionLibrary|ReadLinearPixelfromBufferBilinear (Variables|Default|GetHeightmapReadback) (Utilities|Struct|MakeIntPoint _width _height) (Math|Vector2D|MakeVector2D _x _y)))
      (return (+ (.Z (Math|Vector|BreakVector (Transformation|GetWorldLocation (Variables|Default|GetPlane)))) (* (+ (.R (Math|Color|BreakColor _returnvalue_7)) _zeropoint) _heightmultiplier))))))

(fn DrawHeightmap
  (bind _heightmaprendertarget (Variables|Default|GetHeightmapRenderTarget))
  (Utilities|IsValid _heightmaprendertarget
    (:Is%20Valid
      (bind (_canvas _size _context) (Rendering|BeginDrawCanvastoRenderTarget _heightmaprendertarget))
      (Utilities|FlowControl|Sequence
        (:then_0
          (Canvas|DrawMaterial :self _canvas :RenderMaterial (Variables|Default|GetHeightmapMaterial) :ScreenSize _size))
        (:then_1
          (Rendering|EndDrawCanvastoRenderTarget _context))))))

(fn SetupHeightmapRenderTarget
  (bind _heightmapresolution (Variables|Default|GetHeightmapResolution))
  (bind (_x _y) (Math|Vector2D|BreakVector2D _heightmapresolution))
  (bind _returnvalue (CanvasRenderTarget2D|CreateCanvasRenderTarget2D "/Script/Engine.CanvasRenderTarget2D" (Math|Float|Truncate _x) (Math|Float|Truncate _y)))
  (Variables|/Script/Engine.Texture|SetCompressionSettings _returnvalue "TC_Grayscale")
  (bind _output_get (Variables|Default|SetHeightmapRenderTarget _returnvalue))
  (return _output_get))

(fn SetupSeaPlaneMID
  (bind _seaparameters (Variables|Default|GetSeaParameters))
  (bind (_heightmaprange _heightmultiplier _zeropoint _tesselationmultiplier) (Utilities|Struct|BreakSeaPlaneParameters _seaparameters))
  (bind _returnvalue (Rendering|Material|CreateDynamicMaterialInstance (Variables|Default|GetPlane) 0 (Variables|Default|GetSeaPlaneMaterial) :!class /Script/Engine.PrimitiveComponent))
  (bind _output_get (Variables|Default|SetSeaPlaneMID _returnvalue))
  (Rendering|Material|SetScalarParameterValue _output_get "Heightmap Range" _heightmaprange :!class /Script/Engine.MaterialInstanceDynamic)
  (Rendering|Material|SetScalarParameterValue _output_get "Height Multiplier" _heightmultiplier :!class /Script/Engine.MaterialInstanceDynamic)
  (Rendering|Material|SetScalarParameterValue _output_get "Zero Point" _zeropoint :!class /Script/Engine.MaterialInstanceDynamic)
  (Rendering|Material|SetScalarParameterValue _output_get "Tesselation Multiplier" _tesselationmultiplier :!class /Script/Engine.MaterialInstanceDynamic)
  (return _output_get))