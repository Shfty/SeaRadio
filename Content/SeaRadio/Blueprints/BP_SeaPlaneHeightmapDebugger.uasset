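; BP_SeaPlaneHeightmapDebugger is a debug actor that visualizes the sea plane's height as a grid of debug spheres.
; From its own location it steps over a square grid spaced by GridSize, asks the SeaPlane actor for the height at each point, and draws a sphere there.
; Tick redraws the spheres every frame, while the Construction Script flushes persistent lines and draws long-lived spheres for preview.
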(event Custom|DrawDebug
  (params (Duration :type Float%20%28single-precision%29))
  (for _index (range 0 16)
    (for _index_2 (range 0 16)
      (bind _seaplaneactor (Utilities|GetSeaPlaneActor)
        (:Success
          (bind _height (Default|GetHeightatWorldLocation _seaplaneactor (+ (* (Math|Vector|MakeVector (Math|Conversions|ToFloat(Integer) _index) (Math|Conversions|ToFloat(Integer) _index_2) 0.0) (Variables|Default|GetGridSize)) (Transformation|GetActorLocation))))
          (Rendering|Debug|DrawDebugSphere (Math|Vector|MakeVector (.X (Math|Vector|BreakVector (+ (* (Math|Vector|MakeVector (Math|Conversions|ToFloat(Integer) _index) (Math|Conversions|ToFloat(Integer) _index_2) 0.0) (Variables|Default|GetGridSize)) (Transformation|GetActorLocation)))) (.Y (Math|Vector|BreakVector (+ (* (Math|Vector|MakeVector (Math|Conversions|ToFloat(Integer) _index) (Math|Conversions|ToFloat(Integer) _index_2) 0.0) (Variables|Default|GetGridSize)) (Transformation|GetActorLocation)))) _height) (* (Variables|Default|GetGridSize) 0.25) 4 "(R=0.639431,G=0.000000,B=1.000000,A=1.000000)" Duration))))))

(event EventTick
  (params (DeltaSeconds :type Float%20%28single-precision%29))
  (CallFunction|DrawDebug 0.0))

(fn ConstructionScript
  (Rendering|Debug|FlushPersistentDebugLines)
  (CallFunction|DrawDebug 1e+13))