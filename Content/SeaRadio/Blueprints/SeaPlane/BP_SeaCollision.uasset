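; BP_SeaCollision provides CPU-side sea height queries over a section of the sea plane.
; Each tick, C++ helpers read that section of the SeaPlane's heightmap render target into a float color buffer.
; The construction script sizes its Box from the section's pixel size.
; GetHeightAtWorldLocation maps world position to box UV, bilinearly samples the buffer, then applies the SeaPlane's zero point, height multiplier and actor Z.
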(event EventTick
  (params (DeltaSeconds :type Float%20%28single-precision%29))
  (bind _sectionsize (Variables|Default|GetSectionSize))
  (bind _sectionoffset (Variables|Default|GetSectionOffset))
  (bind (_x _y) (Math|Vector2D|BreakVector2D _sectionoffset))
  (bind _returnvalue (+ _sectionoffset _sectionsize))
  (bind (_x_2 _y_2) (Math|Vector2D|BreakVector2D _returnvalue))
  ;[1 1 1] Use C++ to read floating point color array back from render texture for later use
  (bind _seaplaneactor (Utilities|GetSeaPlaneActor)
    (:Success
      (Utilities|IsValid (Variables|/Game/SeaRadio/Blueprints/SeaPlane/BP_SeaPlane.BP_SeaPlane_C|GetHeightmapRenderTarget _seaplaneactor)
        (:Is%20Valid
          (bind _returnvalue_2 (Class|RenderTextureFunctionLibrary|ReadLinearPixelBufferRect (Variables|/Game/SeaRadio/Blueprints/SeaPlane/BP_SeaPlane.BP_SeaPlane_C|GetHeightmapRenderTarget _seaplaneactor) (Math|Float|Truncate _x) (Math|Float|Truncate _y) (Math|Float|Truncate _x_2) (Math|Float|Truncate _y_2)))
          (Variables|Default|SetHeightmapReadback _returnvalue_2))))))

(fn ConstructionScript
  (bind _sectionsize (Variables|Default|GetSectionSize))
  (bind _returnvalue (* _sectionsize 195.3))
  (bind (_x _y) (Math|Vector2D|BreakVector2D _returnvalue))
  (Components|Box|SetBoxExtent (Variables|Default|GetBox) (Math|Vector|MakeVector _x _y 5e+03) false))

(fn GetHeightatWorldLocation
  (params (InputPin :type Vector))
  (bind _returnvalue (Transformation|GetActorLocation))
  (bind _sectionsize (Variables|Default|GetSectionSize))
  (bind _box (Variables|Default|GetBox))
  (bind (_x _y) (Math|Vector2D|BreakVector2D _sectionsize))
  (bind _returnvalue_2 (Components|Box|GetScaledBoxExtent _box))
  (bind _returnvalue_3 (- _returnvalue _returnvalue_2))
  (bind _returnvalue_4 (* _returnvalue_2 2.0))
  (bind _returnvalue_5 (- InputPin _returnvalue_3))
  (bind _returnvalue_6 (/ _returnvalue_5 _returnvalue_4))
  (bind (_x_2 _y_2) (Math|Vector|BreakVector _returnvalue_6))
  (bind _seaplaneactor (Utilities|GetSeaPlaneActor)
    (:Success
      (bind _returnvalue_7 (Class|RenderTextureFunctionLibrary|ReadLinearPixelfromBufferBilinear (Variables|Default|GetHeightmapReadback) (Utilities|Struct|MakeIntPoint (Math|Float|Truncate _x) (Math|Float|Truncate _y)) (Math|Vector2D|MakeVector2D _x_2 _y_2)))
      (return (+ (.Z (Math|Vector|BreakVector _returnvalue)) (* (+ (.R (Math|Color|BreakColor _returnvalue_7)) (.ZeroPoint (Utilities|Struct|BreakSeaPlaneParameters (Variables|/Game/SeaRadio/Blueprints/SeaPlane/BP_SeaPlane.BP_SeaPlane_C|GetSeaPlaneParameters _seaplaneactor)))) (.HeightMultiplier (Utilities|Struct|BreakSeaPlaneParameters (Variables|/Game/SeaRadio/Blueprints/SeaPlane/BP_SeaPlane.BP_SeaPlane_C|GetSeaPlaneParameters _seaplaneactor)))))))))