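; Buoyancy point component that floats its owning actor on the sea surface provided by BP_SeaPlane.
; Each tick it queries the first BP_SeaPlane found for the height at its own location and sets IsSubmerged.
; It applies an upward impulse there to the owner's root primitive, proportional to depth and divided by the owner's count of these components.
; The impulse is not scaled by delta time.
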(event EventTick
  (params (DeltaSeconds :type Float%20%28single-precision%29))
  (bind _returnvalue (Components|GetOwner))
  (bind _returnvalue_2 (Transformation|GetWorldLocation))
  ;[1 1 1] Tick handler
  ;[1 1 1] Find sea plane actor
  (bind _outactors (Actor|GetAllActorsOfClass "/Game/SeaRadio/Blueprints/BP_SeaPlane.BP_SeaPlane_C"))
  (if (> (Utilities|Array|Length _outactors) 0)
    ;[1 1 1] Check how submerged we are, update flag and apply buoyancy force
    (bind _height (Default|GetHeightatWorldLocation (Utilities|Array|Get(acopy) _outactors) _returnvalue_2))
    (Variables|Default|SetIsSubmerged (> (- _height (.Z (Math|Vector|BreakVector _returnvalue_2))) 0.0))
    (bind _asprimitive_component (Utilities|Casting|CastToPrimitiveComponent (Variables|/Script/Engine.Actor|GetRootComponent _returnvalue)))
    (Physics|AddImpulseatLocation _asprimitive_component (Math|Vector|MakeVector 0.0 0.0 (* (Math|Float|Max(Float) (- _height (.Z (Math|Vector|BreakVector _returnvalue_2))) 0.0) 9.8e+02 (/ 1.0 (Math|Conversions|ToFloat(Integer) (Utilities|Array|Length (Actor|GetComponentsByClass _returnvalue "BP_SeaPlaneBuoyancyComponent_C")))))) (Transformation|GetWorldLocation) "None")))