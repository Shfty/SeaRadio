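; BP_RadioPlayer is a radio player Blueprint that plays audio from a media URL when play begins.
; On BeginPlay it constructs its own MediaPlayer at runtime and assigns it to the MediaSound component, so no MediaPlayer asset is assigned in the graph.
; It then binds OnMediaOpened and opens MediaUrl, starting playback once the media reports it has opened.
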(event Custom|OnMediaOpened
  (params (OpenedUrl :type String))
  ;[1 1 1] When media is opened, play
  (Media|MediaPlayer|Play (Variables|RadioPlayer|State|GetMediaPlayer) :!class /Script/MediaAssets.MediaPlayer))

(event EventBeginPlay
  ;[1 1 1] BeginPlay handler
  (Utilities|FlowControl|Sequence
    (:then_0
      ;[1 1 1] Create media player object and assign it to our media sound component
      (bind _returnvalue (Game|ConstructObjectfromClass "/Script/MediaAssets.MediaPlayer" self))
      (bind _output_get (Variables|RadioPlayer|State|SetMediaPlayer _returnvalue))
      (Variables|/Script/MediaAssets.MediaSoundComponent|SetMediaPlayer (Variables|Default|GetMediaSound) _output_get))
    (:then_1
      ;[1 1 1] Bind OnMediaOpened event, open audio stream URL
      (EventDispatchers|AssignOnMediaOpened (Variables|RadioPlayer|State|GetMediaPlayer) (EventDispatchers|CreateEvent :!event Custom|OnMediaOpened))
      (Class|MediaPlayer|OpenUrl (Variables|RadioPlayer|State|GetMediaPlayer) (Variables|RadioPlayer|GetMediaUrl)))))

(fn ConstructionScript)